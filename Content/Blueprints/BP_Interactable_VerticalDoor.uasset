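; BP_Interactable_VerticalDoor is an interactable door that moves its static mesh vertically when activated.
; Activate calls OpenDoor, which plays the Open timeline from the start.
; Each update adds a local Z offset lerped from zero to OpenHeight by the alpha curve, so movement accumulates per update rather than setting an absolute height.
; It has no closing logic or open-state check.
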(event Custom|OpenDoor
  (bind _alphacurve (Timeline|Open PlayFromStart)
    (:Update
      (Transformation|AddLocalOffset (Variables|Default|GetStaticMesh) (Math|Vector|MakeVector 0.0 0.0 (Math|Float|Lerp 0.0 (Variables|Default|GetOpenHeight) _alphacurve)) false false))))

(event EventBeginPlay
  (|CallParentFunction) ; This node is disabled and will not be called.\nDrag off pins to build functionality.
)

(event Collision|EventActorBeginOverlap
  (params (OtherActor :type Actor%20Object%20Reference))
  (|CallParentFunction OtherActor) ; This node is disabled and will not be called.\nDrag off pins to build functionality.
)

(event EventTick
  (params (DeltaSeconds :type Float%20%28single-precision%29))
  (|CallParentFunction DeltaSeconds) ; This node is disabled and will not be called.\nDrag off pins to build functionality.
)

(event EventActivate
  (CallFunction|OpenDoor))

(fn ConstructionScript
  (|CallParentFunction))