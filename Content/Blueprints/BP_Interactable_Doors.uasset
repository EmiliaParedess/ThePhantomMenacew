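; Interactable double door that slides its left and right panels apart when activated.
; Activate calls OpenDoor, which plays the Close timeline and adds a curve-scaled local offset to each panel on every update, so movement accumulates rather than interpolating between fixed positions.
; CloseDoor reverses the timeline but nothing here calls it, as the three-second delay after opening leads nowhere.
; Closed positions cached at BeginPlay feed no live logic.
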(event Custom|OpenDoor
  (Variables|Default|Setopen true)
  (bind _alphacurve (Timeline|Close Play)
    (:Update
      (Transformation|AddLocalOffset (Variables|Default|GetDoorLeft) (Math|Vector|Lerp(Vector) "0, 0, 0" (Variables|Default|GetOpenPositionLeft) _alphacurve) false false)
      (Transformation|AddLocalOffset (Variables|Default|GetDoorRight) (Math|Vector|Lerp(Vector) "0, 0, 0" (Variables|Default|GetOpenPositionRight) _alphacurve) false false))
    (:Finished
      (if (Variables|Default|Getopen)
        (Utilities|FlowControl|Delay 3.0)))))

(event Custom|CloseDoor
  (bind _alphacurve (Timeline|Close Reverse)
    (:Update
      (Transformation|AddLocalOffset (Variables|Default|GetDoorLeft) (Math|Vector|Lerp(Vector) "0, 0, 0" (Variables|Default|GetOpenPositionLeft) _alphacurve) false false)
      (Transformation|AddLocalOffset (Variables|Default|GetDoorRight) (Math|Vector|Lerp(Vector) "0, 0, 0" (Variables|Default|GetOpenPositionRight) _alphacurve) false false))
    (:Finished
      (if (Variables|Default|Getopen)
        (Utilities|FlowControl|Delay 3.0)))))

(event EventBeginPlay
  (|CallParentFunction)
  (bind _output_get (Variables|Default|SetClosePositionLeft (Transformation|GetWorldLocation (Variables|Default|GetDoorLeft))))
  (bind _output_get_2 (Variables|Default|SetClosePositionRight (Transformation|GetWorldLocation (Variables|Default|GetDoorRight)))))

(event Collision|EventActorBeginOverlap
  (params (OtherActor :type Actor%20Object%20Reference))
  (|CallParentFunction OtherActor) ; This node is disabled and will not be called.\nDrag off pins to build functionality.
)

(event EventTick
  (params (DeltaSeconds :type Float%20%28single-precision%29))
  (|CallParentFunction DeltaSeconds) ; This node is disabled and will not be called.\nDrag off pins to build functionality.
)

(event EventActivate
  (CallFunction|OpenDoor))

(fn ConstructionScript
  (|CallParentFunction))